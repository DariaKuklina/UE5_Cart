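; BP_Cart is a cart actor that travels along an array of splines, one spline per move event from BP_PlayerController.
; Each event increments a queue count, and Tick interpolates a normalized time at constant speed to set location and rotation from the current spline.
; Completed splines decrement the queue, with the index advancing and wrapping to the first.
; Per-frame displacement feeds Speed in ABP_Cart for animation.
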(event Custom|OnMoveCart
  (bind _result (Math|Integer|IncrementInt (Variables|Default|GetSplinesToComplete))
    (:%20%20
      (if (and (== _result 1) (== (Variables|Default|GetTime) 1.0))
        (CallFunction|SetNextSpline)))))

(event EventBeginPlay
  (bind _asbp_player_controller (Utilities|Casting|CastToBP_PlayerController (Game|GetPlayerController 0)))
  (EventDispatchers|BindEventtoMoveCart _asbp_player_controller (delegate Custom|OnMoveCart))
  (Variables|Default|SetLastActorLocation (Transformation|GetActorLocation)))

(event EventTick
  (params (DeltaSeconds :type Float%20%28single-precision%29))
  (CallFunction|CalculateCartMovement)
  (CallFunction|UpdateAnimation))

(fn ConstructionScript)

(fn MoveCart
  (bind _time (Variables|Default|GetTime))
  (bind _splines (Variables|Default|GetSplines))
  (bind _currentspline (Variables|Default|GetCurrentSpline))
  (bind _time_2 (Variables|Default|GetTime))
  (bind _output (Utilities|Array|Get(acopy) _splines _currentspline))
  (bind _spline (Variables|/Game/Blueprints/BP_Spline.BP_Spline_C|GetSpline _output))
  (bind _returnvalue (Spline|GetLocationatTime _spline _time_2 "World" false))
  (bind _returnvalue_2 (Class|SplineComponent|GetDirectionatTime _spline _time "World" false))
  (bind _returnvalue_3 (Math|Conversions|RotationFromXVector _returnvalue_2))
  (Variables|Default|SetLastActorLocation (Transformation|GetActorLocation))
  (Transformation|SetActorLocation (Math|Vector|MakeVector (.x _returnvalue) (.y _returnvalue) (.z _returnvalue)) false false)
  (Transformation|SetActorRotation (Math|Rotator|MakeRotator (.roll _returnvalue_3) (.pitch _returnvalue_3) (.yaw _returnvalue_3))))

(fn CalculateCartMovement
  (if (> (Variables|Default|GetSplinesToComplete) 0)
    (Variables|Default|SetTime (Math|Float|Clamp(Float) (Math|Interpolation|FInterptoConstant (Variables|Default|GetTime) 1.0 (Utilities|Time|GetWorldDeltaSeconds) (Variables|Default|GetCartSpeed))))
    (CallFunction|MoveCart)
    (if (== (Variables|Default|GetTime) 1.0)
      (Variables|Default|SetSplinesToComplete (Math|Integer|Max(Integer) (- (Variables|Default|GetSplinesToComplete) 1)))
      (if (> (Variables|Default|GetSplinesToComplete) 0)
        (CallFunction|SetNextSpline)
        (else
          (Variables|Default|SetLastActorLocation (Transformation|GetActorLocation)))))))

(fn UpdateAnimation
  (bind _asabp_cart (Utilities|Casting|CastToABP_Cart (Components|SkeletalMesh|GetAnimInstance (Variables|Default|GetSkeletalMesh))))
  (Variables|/Game/Blueprints/ABP_Cart.ABP_Cart_C|SetSpeed _asabp_cart (Math|Vector|VectorLength (- (Transformation|GetActorLocation) (Variables|Default|GetLastActorLocation)))))

(fn SetNextSpline
  (Variables|Default|SetCurrentSpline (Math|Integer|SelectInt 0 (+ (Variables|Default|GetCurrentSpline) 1) (> (+ (Variables|Default|GetCurrentSpline) 1) (- (Utilities|Array|Length (Variables|Default|GetSplines)) 1))))
  (Variables|Default|SetTime 0.0))